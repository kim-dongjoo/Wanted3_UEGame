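; Player character Blueprint with Enhanced Input movement, look and a weapon-based montage combo attack.
; A collected weapon attaches to the WeaponPosition socket and enables attacking, while movement only applies in the Idle state.
; Attack starts the montage from Idle, or queues NextCombo from the current section when already attacking.
; OnAttackEnd restores Idle, and attack check begin/end events are forwarded to the weapon.
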(event `self.ReceiveBeginPlay`
  (`EnhancedInputSubsystemInterface.AddMappingContext` (pcsubsystem `EnhancedInputLocalPlayerSubsystem` (`GameplayStatics.GetPlayerController` 0)) "/Game/Blueprint/Inputs/IMC_Default.IMC_Default" 0 (struct)))

(event `EnhancedInput|/Game/Blueprint/Inputs/Actions/IA_Move`
  (params (ActionValue :type "Vector2D Structure") (ElapsedSeconds :type "Float (double-precision)") (TriggeredSeconds :type "Float (double-precision)") (InputAction :type "InputAction Object Reference" :default "/Game/Blueprint/Inputs/Actions/IA_Move.IA_Move"))
  (bind (_returnvalue_roll _returnvalue_pitch _returnvalue_yaw) (`KismetMathLibrary.BreakRotator` (`self.GetControlRotation`)))
  (:`Triggered`
    (switch `/Game/Blueprint/Character/ECharacterState` (`self.State`)
      (:`NewEnumerator0`
        (`self.AddMovementInput` (* (`KismetMathLibrary.GetForwardVector` (`KismetMathLibrary.MakeRotator` 0.0 0.0 _returnvalue_yaw)) ActionValue_Y))
        (`self.AddMovementInput` (* (`KismetMathLibrary.GetRightVector` (`self.GetControlRotation`)) ActionValue_X))))))

(event `EnhancedInput|/Game/Blueprint/Inputs/Actions/IA_Look`
  (params (ActionValue :type "Vector2D Structure") (ElapsedSeconds :type "Float (double-precision)") (TriggeredSeconds :type "Float (double-precision)") (InputAction :type "InputAction Object Reference" :default "/Game/Blueprint/Inputs/Actions/IA_Look.IA_Look"))
  (:`Triggered`
    (`self.AddControllerYawInput` ActionValue_X)
    (`self.AddControllerPitchInput` ActionValue_Y)))

(event `EnhancedInput|/Game/Blueprint/Inputs/Actions/IA_Attack`
  (params (ActionValue :type Boolean) (ElapsedSeconds :type "Float (double-precision)") (TriggeredSeconds :type "Float (double-precision)") (InputAction :type "InputAction Object Reference" :default "/Game/Blueprint/Inputs/Actions/IA_Attack.IA_Attack"))
  (:`Triggered`
    (`self.Attack`)))

(event `Attack`
  (if (`self.HasWeapon`)
    (switch `/Game/Blueprint/Character/ECharacterState` (`self.State`)
      (:`NewEnumerator0`
        (set `self.State` "NewEnumerator1")
        (`self.PlayAnimMontage` "/Game/InfinityBladeWarriors/Animations/WarriorAttack1_Montage.WarriorAttack1_Montage" 1.0 "Attack1"))
      (:`NewEnumerator1`
        (switch `name` (`AnimInstance.Montage_GetCurrentSection` (`SkeletalMeshComponent.GetAnimInstance` (`self.Mesh`)) null)
          (:`Attack1`
            (set `self.NextCombo` "Attack2"))
          (:`Attack2`
            (set `self.NextCombo` "Attack3"))
          (:`Attack3`
            (set `self.NextCombo` "Attack4")))))))

(event `OnAttackEnd`
  (set `self.State` "NewEnumerator0"))

(event `OnWeaponCollected`
  (params (WeaponActor :type "/Game/Blueprint/Character/BP_Weapon Object Reference"))
  ; 무기 수집
  (`self.SetOwner` WeaponActor self)
  (bind _returnvalue (`self.K2_AttachToComponent` WeaponActor (`self.Mesh`) "WeaponPosition" "SnapToTarget" "SnapToTarget" "KeepRelative" true))
  (set `self.HasWeapon` _returnvalue)
  (set `self.Weapon` (cast `/Game/Blueprint/Character/BP_Weapon` WeaponActor :!pure true)))

(event `OnAttackCheckBegin`
  (`/Game/Blueprint/Character/BP_Weapon.OnAttackCheckBegin` (`self.Weapon`)))

(event `OnAttackCheckEnd`
  (`/Game/Blueprint/Character/BP_Weapon.OnAttackCheckEnd` (`self.Weapon`)))

(fn `UserConstructionScript`)