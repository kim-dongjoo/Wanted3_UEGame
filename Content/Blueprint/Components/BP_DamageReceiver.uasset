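; Damage receiver component that tracks its owner's health and reports changes and death.
; Health starts at MaxHealth on BeginPlay, and OnDamageTaken subtracts damage, clamping the result between zero and a hardcoded 100 rather than MaxHealth.
; At zero it calls OnDead; otherwise it calls OnHealthChanged with current and maximum health.
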(event `self.ReceiveBeginPlay`
  (set `self.Health` (`self.MaxHealth`)))

(event `OnDamageTaken`
  (params (Damage :type "Float (double-precision)"))
  (bind _output_get (set `self.Health` (`KismetMathLibrary.FClamp` (- (`self.Health`) Damage) 0.0 100.0)))
  (if (== _output_get 0.0)
    (`self.OnDead`)
    (else
      (`self.OnHealthChanged` (`self.Health`) (`self.MaxHealth`)))))