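; BP_MonsterBear is a bear monster that takes damage, shows hit feedback and handles its own death.
; AnyDamage passes damage to the DamageReceiver component, then restarts a timeline that drives HitValue on a dynamic stone-bear material.
; The same timeline update refreshes the WBP_HP bar from the current health ratio, while OnHealthChanged is bound but empty.
; On death it disables capsule collision and enters a final state that SetState never leaves.
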(event `SetState`
  (params (NewState :type "/Game/Blueprint/Monster/EMonsterState Enum" :default "NewEnumerator0"))
  (if (`|EnumInequality` (`self.State`) "NewEnumerator3")
    (if (`|EnumInequality` NewState (`self.State`))
      (set `self.State` NewState))))

(event `self.ReceiveBeginPlay`
  (bind _returnvalue (`PrimitiveComponent.CreateDynamicMaterialInstance` (`self.Mesh`) 0 "/Game/InfinityBladeAdversaries/Enemy/Enemy_Bear/Materials/M_Bear_Stone_Inst.M_Bear_Stone_Inst" "None"))
  (set `self.Dynamic Instance` _returnvalue)
  (add `/Game/Blueprint/Components/BP_DamageReceiver.OnDead` (`self.DamageReceiver`) (delegate `OnDead`))
  (add `/Game/Blueprint/Components/BP_DamageReceiver.OnHealthChanged` (`self.DamageReceiver`) (delegate `OnHealthChanged`)))

(event `OnDead`
  (`PrimitiveComponent.SetCollisionEnabled` (`self.CapsuleComponent`) "NoCollision")
  (`self.SetState` "NewEnumerator3"))

(event `OnHealthChanged`
  (params (Health :type "Float (double-precision)") (MaxHealth :type "Float (double-precision)")))

(event `self.ReceiveAnyDamage`
  (params (Damage :type "Float (single-precision)") (DamageType :type "DamageType Object Reference") (InstigatedBy :type "Controller Object Reference") (DamageCauser :type "Actor Object Reference"))
  (bind _damagereceiver (`self.DamageReceiver`))
  (`/Game/Blueprint/Components/BP_DamageReceiver.OnDamageTaken` (`self.DamageReceiver`) Damage)
  (bind (_direction _value) (`Timeline|HitEffect` :!via `PlayFromStart`)
    (:`Update`
      (`MaterialInstanceDynamic.SetScalarParameterValue` (`self.Dynamic Instance`) "HitValue" _value)
      (bind _aswbp_hp (cast `/Game/UI/WBP/WBP_HP` (`WidgetComponent.GetUserWidgetObject` (`self.HPBar`))))
      (`/Game/UI/WBP/WBP_HP.SetHPPercent` _aswbp_hp (`KismetMathLibrary.FClamp` (/ (`/Game/Blueprint/Components/BP_DamageReceiver.Health` _damagereceiver) (`/Game/Blueprint/Components/BP_DamageReceiver.MaxHealth` _damagereceiver)))))))

(fn `UserConstructionScript`)